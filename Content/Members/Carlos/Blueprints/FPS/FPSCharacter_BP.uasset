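; FPS soldier character Blueprint that the third-person character can possess when in range.
; A ControlBox overlap with BP_ThirdPersonCharacter sets CanPossess.
; Tick swaps first-person hands and soldier body by scaling each to zero or one based on ImPossessed.
; SelectEnemy clears custom depth on every instance, then enables it on this mesh if possessable, marking a single selected target.
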(event `self.ReceiveBeginPlay`
  (bind _output_get (set `self.HandsMesh` (`self.HandsMeshComp`)))
  (`SceneComponent.SetWorldScale3D` _output_get (0.0 0.0 0.0))
  (set `self.SoldierMesh` (`self.Mesh`)))

(event `self.ReceiveTick`
  (params (DeltaSeconds :type "Float (single-precision)"))
  ;[1 1 1] Escondemos o mostramos mesh
  (if (`self.ImPossessed`)
    (`SceneComponent.SetWorldScale3D` (`self.HandsMesh`) (1.0 1.0 1.0))
    (`SceneComponent.SetWorldScale3D` (`self.SoldierMesh`) (0.0 0.0 0.0))
    (else
      (`SceneComponent.SetWorldScale3D` (`self.HandsMesh`) (0.0 0.0 0.0))
      (`SceneComponent.SetWorldScale3D` (`self.SoldierMesh`) (1.0 1.0 1.0))))
  (if (`self.IsDead`)
    _))

(event `self.ControlBox.OnComponentBeginOverlap`
  (params (OverlappedComponent :type "PrimitiveComponent Object Reference") (OtherActor :type "Actor Object Reference") (OtherComp :type "PrimitiveComponent Object Reference") (OtherBodyIndex :type Integer) (bFromSweep :type Boolean) (SweepResult :type "HitResult Structure (by ref)"))
  (cast `/Game/ThirdPerson/Blueprints/BP_ThirdPersonCharacter` OtherActor)
  (set `self.CanPossess` true))

(event `self.ControlBox.OnComponentEndOverlap`
  (params (OverlappedComponent :type "PrimitiveComponent Object Reference") (OtherActor :type "Actor Object Reference") (OtherComp :type "PrimitiveComponent Object Reference") (OtherBodyIndex :type Integer))
  (cast `/Game/ThirdPerson/Blueprints/BP_ThirdPersonCharacter` OtherActor)
  (set `self.CanPossess` false))

(fn `SelectEnemy`
  (bind _outactors (`GameplayStatics.GetAllActorsOfClass` "FPSCharacter_BP_C"))
  (for _array_element _outactors
    (`PrimitiveComponent.SetRenderCustomDepth` (`Character.Mesh` _array_element) false))
  (if (`self.CanPossess`)
    (`PrimitiveComponent.SetRenderCustomDepth` (`self.Mesh`) true)))

(fn `UserConstructionScript`)